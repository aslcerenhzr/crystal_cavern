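; BP_Win is a level-exit actor that advances the player to the next level once all crystals are collected.
; On player overlap, it checks for remaining BP_Crystal actors and prints a debug message if any exist.
; Otherwise it finds the current level in the LevelName array and opens the following entry by name.
; On the last listed level it only prints a message.
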(event `self.ReceiveActorBeginOverlap`
  (params (OtherActor :type "Actor Object Reference"))
  (`/Game/Libraries/CC_Macro.IsPlayer2` OtherActor
    (:`IsPlayer`
      (if (`self.Any Crystal Remaning` null)
        (`KismetSystemLibrary.PrintString` "bitmedi")
        (else
          (`self.Complete Level`))))))

(fn `Any Crystal Remaning`
  (params (Actor :type "Object Object Reference"))
  (returns (NewParam :type Boolean))
  (bind _outactors (`GameplayStatics.GetAllActorsOfClass` "/Game/Blueprints/Actors/BP_Crystal.BP_Crystal_C"))
  (return (> (`KismetArrayLibrary.Array_Length` _outactors) 0)))

(fn `Complete Level`
  (returns (NewParam :type Boolean))
  (if (`self.IsLevelFinal`)
    (`KismetSystemLibrary.PrintString` "butun crystalleri toplamadın")
    (else
      (`self.Load Next Level`))))

(fn `Get Current Level Index`
  (returns (NewParam :type Integer))
  (bind _returnvalue (`GameplayStatics.GetCurrentLevelName` true))
  (return (`KismetArrayLibrary.Array_Find` (`self.Level Name`) (`KismetStringLibrary.Conv_StringToName` _returnvalue))))

(fn `GetNextLevelName`
  (returns (Output :type Name))
  (return (`|GetArrayItem` (`self.Level Name`) (+ (`self.Get Current Level Index`) 1))))

(fn `IsLevelFinal`
  (returns (ReturnValue :type Boolean))
  (return (== (`KismetArrayLibrary.Array_LastIndex` (`self.Level Name`)) (`self.Get Current Level Index`))))

(fn `Load Next Level`
  (`GameplayStatics.OpenLevel` (`self.GetNextLevelName`)))

(fn `UserConstructionScript`)