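; BP_Player is a player Blueprint that rolls a mesh with torque and restarts the level when hurt.
; Forward/backward and right/left input axes feed one acceleration-change torque node on StaticMeshPlayer, scaled by AccelerationNumber.
; Any damage calls Restart, which uses DoOnce to fade the camera out, wait briefly and reload the current level.
; BeginPlay fades the camera in.
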(event `InputAxis|Movr Forwards/Backwards`
  (params (AxisValue :type "Float (single-precision)"))
  (bind _acceleration_number (`self.Acceleration Number`))
  (`PrimitiveComponent.AddTorqueInRadians` (`self.StaticMesh_Player`) (`KismetMathLibrary.MakeVector` (* AxisValue _acceleration_number) (* (stale `InputAxis|Move Right/Left` AxisValue) _acceleration_number)) "None" true :!label _label))

(event `self.ReceiveBeginPlay`
  (`PlayerCameraManager.StartCameraFade` :`self` (`GameplayStatics.GetPlayerCameraManager` 0) :`FromAlpha` 1.0 :`Duration` 5.0))

(event `self.ReceiveAnyDamage`
  (params (Damage :type "Float (single-precision)") (DamageType :type "DamageType Object Reference") (InstigatedBy :type "Controller Object Reference") (DamageCauser :type "Actor Object Reference"))
  (`/Engine/EditorBlueprintResources/StandardMacros.DoOnce` false
    (:`Completed`
      (`PlayerCameraManager.StartCameraFade` :`self` (`GameplayStatics.GetPlayerCameraManager` 0) :`ToAlpha` 1.0 :`Duration` 1.0 :`bHoldWhenFinished` true)
      (`KismetSystemLibrary.Delay` 1.5)
      (bind _returnvalue (`GameplayStatics.GetCurrentLevelName` true))
      (`GameplayStatics.OpenLevel` (`KismetStringLibrary.Conv_StringToName` _returnvalue)))))

(event `InputAxis|Move Right/Left`
  (params (AxisValue :type "Float (single-precision)"))
  (goto _label))

(fn `UserConstructionScript`)