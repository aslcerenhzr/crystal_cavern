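; BP_Player is the player pawn, a physics-driven mesh that collects crystals and restarts the level when damaged.
; Both movement axes feed one torque node that applies the scaled input equally to X and Y.
; AddCrystal and a timed Warning event update the GameUI widget created on BeginPlay, which also fades the camera in.
; Damage triggers a one-shot fade-out and level reload, while Escape opens MenuLevel.
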(event `InputAxis|Movr Forwards/Backwards`
  (params (AxisValue :type "Float (single-precision)"))
  (bind _acceleration_number (`self.Acceleration Number`))
  (`PrimitiveComponent.AddTorqueInRadians` (`self.StaticMesh_Player`) (`KismetMathLibrary.MakeVector` (* AxisValue _acceleration_number) (* (stale `InputAxis|Move Right/Left` AxisValue) _acceleration_number)) "None" true :!label _label))

(event `self.ReceiveBeginPlay`
  (bind _returnvalue (`|CreateWidget` "/Game/UI/WBP_GameUI.WBP_GameUI_C"))
  (bind _output_get (set `self.GameUIREF` _returnvalue))
  (`UserWidget.AddToViewport` _output_get 0)
  (`PlayerCameraManager.StartCameraFade` :`self` (`GameplayStatics.GetPlayerCameraManager` 0) :`FromAlpha` 1.0 :`Duration` 5.0))

(event `self.ReceiveAnyDamage`
  (params (Damage :type "Float (single-precision)") (DamageType :type "DamageType Object Reference") (InstigatedBy :type "Controller Object Reference") (DamageCauser :type "Actor Object Reference"))
  (`/Engine/EditorBlueprintResources/StandardMacros.DoOnce` false
    (:`Completed`
      (`PlayerCameraManager.StartCameraFade` :`self` (`GameplayStatics.GetPlayerCameraManager` 0) :`ToAlpha` 1.0 :`Duration` 1.0 :`bHoldWhenFinished` true)
      (`KismetSystemLibrary.Delay` 1.5)
      (bind _returnvalue (`GameplayStatics.GetCurrentLevelName` true))
      (`GameplayStatics.OpenLevel` (`KismetStringLibrary.Conv_StringToName` _returnvalue))
      (set `self.NumberofCrystal` 0))))

(event `InputAxis|Move Right/Left`
  (params (AxisValue :type "Float (single-precision)"))
  (goto _label))

(event `Key|Escape`
  (params (Key :type "Key Structure"))
  (:`Pressed`
    (`GameplayStatics.OpenLevel` "MenuLevel")))

(event `Warning`
  (bind _warning (`/Game/UI/WBP_GameUI.warning` (`self.GameUIREF`)))
  (`Widget.SetVisibility` _warning "Visible")
  (`KismetSystemLibrary.Delay` 2.0)
  (`Widget.SetVisibility` _warning "Hidden"))

(fn `AddCrystal`
  (bind _output_get (set `self.NumberofCrystal` (+ (`self.NumberofCrystal`) 1.0)))
  (`TextBlock.SetText` (`/Game/UI/WBP_GameUI.NumberOfCrystal` (`self.GameUIREF`)) (`KismetTextLibrary.Conv_StringToText` (`KismetStringLibrary.Concat_StrStr` "Crystal:" (`KismetStringLibrary.Conv_IntToString` _output_get)))))

(fn `UserConstructionScript`)