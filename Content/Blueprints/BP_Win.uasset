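; BP_Win is the level exit actor that advances the game when the player overlaps it.
; If any BP_Crystal actors remain in the level, it calls Warning on BP_Player instead of completing.
; Otherwise it finds the current level in its ordered LevelName array and opens the next entry, or MenuLevel after the last one.
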(event `self.ReceiveActorBeginOverlap`
  (params (OtherActor :type "Actor Object Reference"))
  (bind _returnvalue (`/Game/Libraries/CC_Macro.IsPlayer2` OtherActor)
    (:`IsPlayer`
      (if (`self.Any Crystal Remaning` null)
        (bind _asbp_player (cast `/Game/Blueprints/BP_Player` _returnvalue))
        (`/Game/Blueprints/BP_Player.Warning` _asbp_player)
        (else
          (`self.Complete Level`))))))

(fn `Any Crystal Remaning`
  (params (Actor :type "Object Object Reference"))
  (returns (NewParam :type Boolean))
  (bind _outactors (`GameplayStatics.GetAllActorsOfClass` "/Game/Blueprints/Actors/BP_Crystal.BP_Crystal_C"))
  (return (> (`KismetArrayLibrary.Array_Length` _outactors) 0)))

(fn `Complete Level`
  (returns (NewParam :type Boolean))
  (if (`self.IsLevelFinal`)
    (`GameplayStatics.OpenLevel` "MenuLevel")
    (else
      (`self.Load Next Level`))))

(fn `Get Current Level Index`
  (returns (NewParam :type Integer))
  (bind _returnvalue (`GameplayStatics.GetCurrentLevelName` true))
  (return (`KismetArrayLibrary.Array_Find` (`self.Level Name`) (`KismetStringLibrary.Conv_StringToName` _returnvalue))))

(fn `GetNextLevelName`
  (returns (Output :type Name))
  (return (`|GetArrayItem` (`self.Level Name`) (+ (`self.Get Current Level Index`) 1))))

(fn `IsLevelFinal`
  (returns (ReturnValue :type Boolean))
  (return (== (`KismetArrayLibrary.Array_LastIndex` (`self.Level Name`)) (`self.Get Current Level Index`))))

(fn `Load Next Level`
  (`GameplayStatics.OpenLevel` (`self.GetNextLevelName`)))

(fn `UserConstructionScript`)